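; Level-design prop actor that sets its static mesh and builds its material at BeginPlay from exposed-style variables.
; MaterialType selects a Base, Emmissif or Liquid path, each creating a dynamic material instance on slot 0 and pushing its color, scalar and normal-map parameters.
; An optional FreestyleRandomMaterial flag triggers per-type randomization of those parameters before the material is created.
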(event `SpawnMatEmmissif`
  ;[1 1 1] Mat Emmissif : Color ; Light (Power de lumière)
  (bind _returnvalue (`PrimitiveComponent.CreateDynamicMaterialInstance` (`self.StaticMesh`) 0 "/Game/Material/MAT_EMMISSIF_Inst.MAT_EMMISSIF_Inst"))
  (`MaterialInstanceDynamic.SetVectorParameterValue` _returnvalue "Color" (`self.Color`))
  (`MaterialInstanceDynamic.SetScalarParameterValue` _returnvalue "Power" (`self.Light`)))

(event `SpawnMatBase`
  ;[1 1 1] Mat Base : Mouvement = PannerTime ; Normal Map ; Color ; Emmissif ; Specular ; Rough ; Metal
  (bind _returnvalue (`PrimitiveComponent.CreateDynamicMaterialInstance` (`self.StaticMesh`) 0 "/Game/Material/MAT_BASE_Inst.MAT_BASE_Inst"))
  (`MaterialInstanceDynamic.SetTextureParameterValue` _returnvalue "Normal" (`self.Normal`))
  (`MaterialInstanceDynamic.SetScalarParameterValue` _returnvalue "Speed" (`self.PannerTime`))
  (`MaterialInstanceDynamic.SetScalarParameterValue` _returnvalue "Metal" (`self.Metal`))
  (`MaterialInstanceDynamic.SetVectorParameterValue` _returnvalue "Color" (`self.Color`))
  (`MaterialInstanceDynamic.SetScalarParameterValue` _returnvalue "Emmissif" (`self.Emmissif`))
  (`MaterialInstanceDynamic.SetScalarParameterValue` _returnvalue "Rough" (`self.Rough`))
  (`MaterialInstanceDynamic.SetScalarParameterValue` _returnvalue "Specular" (`self.Specular`)))

(event `SpawnMatLiquid`
  ;[1 1 1] Mat Liquide : Normal ; Opacity ; PannerTime ; Color
  (bind _returnvalue (`PrimitiveComponent.CreateDynamicMaterialInstance` (`self.StaticMesh`) 0 "/Game/Material/MAT_WATER_Inst.MAT_WATER_Inst"))
  (`MaterialInstanceDynamic.SetTextureParameterValue` _returnvalue "Normal" (`self.Normal`))
  (`MaterialInstanceDynamic.SetScalarParameterValue` _returnvalue "Opacity" (`self.OpacityValue`))
  (`MaterialInstanceDynamic.SetScalarParameterValue` _returnvalue "PannerTime" (`self.PannerTime`))
  (`MaterialInstanceDynamic.SetVectorParameterValue` _returnvalue "Color" (`self.Color`)))

(event `SpawnMesh`
  (`StaticMeshComponent.SetStaticMesh` (`self.StaticMesh`) (`self.Mesh`)))

(event `self.ReceiveBeginPlay`
  (`self.SpawnMesh`)
  (switch `/Game/Enum/Material` (`self.MaterialType`)
    (:`NewEnumerator0`
      ;[1 1 1] Freestyle Random Material
      (if (`self.FreestyleRandomMaterial`)
        (`self.RandomMat_Base`))
      (`self.SpawnMatBase`))
    (:`NewEnumerator1`
      (if (`self.FreestyleRandomMaterial`)
        (`self.RandomMat_Emissif`))
      (`self.SpawnMatEmmissif`))
    (:`NewEnumerator2`
      (if (`self.FreestyleRandomMaterial`)
        (`self.RandomMat_Liquid`))
      (`self.SpawnMatLiquid`))))

(event `RandomMat_Base`
  ;[1 1 1] RandomMat_Base
  (`|ExecutionSequence`
    (:`then_0`
      (set `self.PannerTime` (`KismetMathLibrary.RandomFloatInRange` 0.0 1.0)))
    (:`then_1`
      (set `self.Color` (make `LinearColor` (`KismetMathLibrary.RandomFloatInRange` 0.0 1.0) (`KismetMathLibrary.RandomFloatInRange` 0.0 1.0) (`KismetMathLibrary.RandomFloatInRange` 0.0 1.0) 1.0)))
    (:`then_2`
      (set `self.Metal` (`KismetMathLibrary.RandomFloatInRange` 0.0 1.0)))
    (:`then_3`
      (set `self.Emmissif` 0.0))
    (:`then_4`
      (set `self.Rough` (`KismetMathLibrary.RandomFloatInRange` 0.0 1.0)))
    (:`then_5`
      (set `self.Specular` (`KismetMathLibrary.RandomFloatInRange` 0.0 1.0)))
    (:`then_6`
      (set `self.Normal` (select `int` (`KismetMathLibrary.RandomIntegerInRange` 0 1) :`0` "/Game/TExtures/N_TEXT_BLOOD_02.N_TEXT_BLOOD_02" :`1` "/Game/TExtures/N_TEXT_METAL.N_TEXT_METAL" :`2` null :!type "Texture Object Reference")))))

(event `RandomMat_Emissif`
  (`|ExecutionSequence`
    (:`then_0`
      (set `self.Color` (make `LinearColor` (`KismetMathLibrary.RandomFloatInRange` 0.0 1.0) (`KismetMathLibrary.RandomFloatInRange` 0.0 1.0) (`KismetMathLibrary.RandomFloatInRange` 0.0 1.0) 1.0)))
    (:`then_1`
      (set `self.Light` (`KismetMathLibrary.RandomFloatInRange` 0.0 25.0)))))

(event `RandomMat_Liquid`
  (`|ExecutionSequence`
    (:`then_0`
      (set `self.OpacityValue` (`KismetMathLibrary.RandomFloatInRange` 0.0 1.0)))
    (:`then_1`
      (set `self.PannerTime` (`KismetMathLibrary.RandomFloatInRange` 0.0 1.0)))
    (:`then_2`
      (set `self.Color` (make `LinearColor` (`KismetMathLibrary.RandomFloatInRange` 0.0 1.0) (`KismetMathLibrary.RandomFloatInRange` 0.0 1.0) (`KismetMathLibrary.RandomFloatInRange` 0.0 1.0) 1.0)))
    (:`then_3`
      (set `self.Normal` (select `int` (`KismetMathLibrary.RandomIntegerInRange` 0 1) :`0` "/Game/TExtures/N_TEXT_BLOOD_02.N_TEXT_BLOOD_02" :`1` "/Game/TExtures/N_TEXT_METAL.N_TEXT_METAL" :`2` null :!type "Texture Object Reference")))))

(fn `UserConstructionScript`)