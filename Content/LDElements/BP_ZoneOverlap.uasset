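; Sphere trigger zone that reskins the sky while it is overlapped.
; Spawn plays one of ten random audio events on Sound3D.
; Begin overlap randomizes the CustomSkySphere's color and material parameters, hiding the swap behind a white fade run through KillBox actors.
; End overlap repeats the fade, restores the white sky and destroys the zone, making it single-use.
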(event `Spawn`
  (`FMODBlueprintStatics.PlayEventAttached` (select `int` (`KismetMathLibrary.RandomIntegerInRange` 0 9) :`0` null :`1` null :`2` null :`3` null :`4` null :`5` null :`6` null :`7` null :`8` null :`9` null :!type "FMODEvent Object Reference") (`self.Sound3D`) "None" (0.0 0.0 0.0) "KeepRelativeOffset"))

(event `self.SphereCollision.OnComponentBeginOverlap`
  (params (OtherActor :type "Actor Object Reference") (OtherComp :type "PrimitiveComponent Object Reference") (OtherBodyIndex :type Integer) (bFromSweep :type Boolean) (SweepResult :type "HitResult Structure (by ref)"))
  (`|ExecutionSequence`
    (:`then_0`
      (bind _outactors (`GameplayStatics.GetAllActorsOfClass` "/Game/LDElements/KillBox.KillBox_C"))
      (`/Game/LDElements/KillBox.WhiteFade` _outactors 0.2 true))
    (:`then_1`
      (`KismetSystemLibrary.Delay` 0.2)
      (`|ExecutionSequence`
        (:`then_0`
          (bind _outactors_2 (`GameplayStatics.GetAllActorsOfClass` "/Game/CustomSkySphere.CustomSkySphere_C"))
          (bind _item (`KismetArrayLibrary.Array_Get` _outactors_2))
          (set `/Game/CustomSkySphere.Material` "/Game/Material/MAT_Sky_Inst.MAT_Sky_Inst" _item)
          (set `/Game/CustomSkySphere.Color` (make `LinearColor` (`KismetMathLibrary.RandomFloatInRange` 0.0 1.0) (`KismetMathLibrary.RandomFloatInRange` 0.0 1.0) (`KismetMathLibrary.RandomFloatInRange` 0.0 1.0) (`KismetMathLibrary.RandomFloatInRange` 0.0 1.0)) _item)
          (set `/Game/CustomSkySphere.Emmissif` (`KismetMathLibrary.RandomFloatInRange` 0.0 0.0) _item)
          (set `/Game/CustomSkySphere.Normal` (select `int` (`KismetMathLibrary.RandomInteger` 2) :`0` "/Game/TExtures/N_TEXT_BLOOD_02.N_TEXT_BLOOD_02" :`1` "/Game/TExtures/N_TEXT_METAL.N_TEXT_METAL" :`2` "/Game/TExtures/N_BrickSmall.N_BrickSmall" :!type "Texture Object Reference") _item)
          (set `/Game/CustomSkySphere.Metal` (`KismetMathLibrary.RandomFloatInRange` 0.0 1.0) _item)
          (set `/Game/CustomSkySphere.Rough` (`KismetMathLibrary.RandomFloatInRange` 0.0 1.0) _item)
          (set `/Game/CustomSkySphere.Specular` (`KismetMathLibrary.RandomFloatInRange` 0.0 1.0) _item)
          (set `/Game/CustomSkySphere.Speed` (`KismetMathLibrary.RandomFloatInRange` 0.0 1.0) _item)
          (`/Game/CustomSkySphere.Set color` _outactors_2))
        (:`then_1`
          (`/Game/LDElements/KillBox.WhiteFade` _outactors 0.2 false))))))

(event `self.SphereCollision.OnComponentEndOverlap`
  (params (OtherActor :type "Actor Object Reference") (OtherComp :type "PrimitiveComponent Object Reference") (OtherBodyIndex :type Integer))
  (`|ExecutionSequence`
    (:`then_0`
      (bind _outactors (`GameplayStatics.GetAllActorsOfClass` "/Game/LDElements/KillBox.KillBox_C"))
      (`/Game/LDElements/KillBox.WhiteFade` _outactors 0.2 true))
    (:`then_1`
      (`KismetSystemLibrary.Delay` 0.2)
      (`|ExecutionSequence`
        (:`then_0`
          (bind _outactors_2 (`GameplayStatics.GetAllActorsOfClass` "/Game/CustomSkySphere.CustomSkySphere_C"))
          (bind _item (`KismetArrayLibrary.Array_Get` _outactors_2))
          (set `/Game/CustomSkySphere.Material` "/Game/Material/WhiteSky_Inst.WhiteSky_Inst" _item)
          (`/Game/CustomSkySphere.KillColor` _item)
          (`self.K2_DestroyActor`))
        (:`then_1`
          (`/Game/LDElements/KillBox.WhiteFade` _outactors 0.2 false))))))

(fn `UserConstructionScript`)